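; Car is a looping traffic hazard that ends the game when the player touches it.
; Each tick it moves along its root's forward vector at Speed without sweeping.
; Once it is farther than Distance from StartPosition, it teleports back to StartPosition to repeat the run.
; On overlap, it casts the other actor to Player and calls GameOver.
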(event EventTick
  (params (DeltaSeconds :type Float%20%28single-precision%29))
  (Transformation|AddActorWorldOffset (* (* DeltaSeconds (Variables|Default|GetSpeed)) (Math|Vector|GetForwardVector (Variables|Default|GetDefaultSceneRoot))))
  (if (> (Math|Vector|Distance(Vector) (Transformation|GetActorLocation) (Variables|Default|GetStartPosition)) (Variables|Default|GetDistance))
    (Transformation|SetActorLocation (Variables|Default|GetStartPosition) false false)))

(event Collision|EventActorBeginOverlap
  (params (OtherActor :type Actor%20Object%20Reference))
  (bind _asplayer (Utilities|Casting|CastToPlayer OtherActor))
  (Default|GameOver _asplayer))

(fn ConstructionScript)