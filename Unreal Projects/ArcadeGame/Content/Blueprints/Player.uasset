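; Player Blueprint for a step-based game, moving in fixed hops forward, left or right and tracking score.
; TryMove shifts a target position, then locks input briefly until a timer re-enables it, while Tick drives MoveComponentTo toward that target.
; BeginPlay creates the score widget, which AddScore updates.
; GameOver shows the end screen and mouse cursor.
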(event EventTick
  (params (DeltaSeconds :type Float%20%28single-precision%29))
  (Components|MoveComponentTo (Variables|Default|GetDefaultSceneRoot) (Variables|Default|GetTargetPos) "0, 0, 0" false false 0.2 false))

(event EventBeginPlay
  (bind _returnvalue (UserInterface|CreateWidget "/Game/Blueprints/ScoreUI.ScoreUI_C"))
  (UserInterface|Viewport|AddtoViewport _returnvalue 0)
  (Variables|Default|SetScoreUI _returnvalue))

(event Input|ActionEvents|InputActionMove_Forward
  (params (Key :type Key%20Structure :default "None"))
  (:Pressed
    (CallFunction|TryMove "100.000000,0.000000,0.000000")))

(event Input|ActionEvents|InputActionMove_Left
  (params (Key :type Key%20Structure :default "None"))
  (:Pressed
    (CallFunction|TryMove "0.000000,-100.000000,0.000000")))

(event Input|ActionEvents|InputActionMove_Right
  (params (Key :type Key%20Structure :default "None"))
  (:Pressed
    (CallFunction|TryMove "0.000000,100.000000,0.000000")))

(fn ConstructionScript)

(fn TryMove
  (params (Direction :type Vector))
  (if (Variables|Default|GetCanMove)
    (Variables|Default|SetTargetPos (+ Direction (Variables|Default|GetTargetPos)))
    (Variables|Default|SetCanMove false)
    (Utilities|Time|SetTimerbyFunctionName 0 "EnableCanMove" 0.3)))

(fn EnableCanMove
  (Variables|Default|SetCanMove true))

(fn GameOver
  (bind _returnvalue (UserInterface|CreateWidget "/Game/Blueprints/EndScreenUI.EndScreenUI_C"))
  (UserInterface|Viewport|AddtoViewport _returnvalue 0)
  (Default|SetGameOverScreen _returnvalue)
  (Variables|/Script/Engine.PlayerController|SetbShowMouseCursor (Game|GetPlayerController 0) true))

(fn AddScore
  (params (ScoreToAdd :type Integer))
  (bind _output_get (Variables|Default|SetScore (+ ScoreToAdd (Variables|Default|GetScore))))
  (Default|UpdateScoreText (Variables|Default|GetScoreUI) _output_get))